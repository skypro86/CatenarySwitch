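; Spawner actor that creates up to twelve BP_Cable actors one at a time, apparently for a catenary switch setup.
; Tick spawns a cable when IsSpawned is false, then sets the flag and increments the count; nothing here clears the flag.
; The count indexes link lengths and drives helper functions that build numbered socket names and location tags.
; Tags pair up per group of four cables, with Long and ExtraLong variants for some later cables.
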(event `self.ReceiveBeginPlay`)

(event `self.ReceiveTick`
  (params (DeltaSeconds :type "Float (single-precision)"))
  (bind _numcablesspawned (`self.NumCablesSpawned`))
  (bind _returnvalue (`KismetStringLibrary.Conv_IntToString` (+ _numcablesspawned 1)))
  (bind _returnvalue_2 (select `int` (/ _numcablesspawned 4) :`0` 1 :`1` 3 :`2` 5))
  (if (`self.isSpawned`)
    _
    (elif (< (`self.NumCablesSpawned`) 12)
      (`|SpawnActorFromClass` "/Game/CatenarySwitch/Art/Industrial/Cable/BP_Cable.BP_Cable_C" (`KismetMathLibrary.MakeTransform` (-5.0 -15.0 5.0) (struct) (1.0 0.5 0.5)) "AdjustIfPossibleButAlwaysSpawn" "MultiplyWithRoot" null 20.0 (`|GetArrayItem` (`self.Lengths`) _numcablesspawned) (`KismetStringLibrary.Conv_StringToName` (`KismetStringLibrary.Concat_StrStr` "Socket_Cable" _returnvalue)) (`KismetStringLibrary.Conv_StringToName` (`KismetStringLibrary.Concat_StrStr` "Socket_Cable" _returnvalue "_2")) (select `bool` (and (> _numcablesspawned 7) (< _numcablesspawned 12)) :`true` (`KismetStringLibrary.Conv_StringToName` (`KismetStringLibrary.Concat_StrStr` "Socket_Cable" _returnvalue "_Long"))) (select `bool` (or (== _numcablesspawned 9) (== _numcablesspawned 10)) :`true` (`KismetStringLibrary.Conv_StringToName` (`KismetStringLibrary.Concat_StrStr` "Socket_Cable" _returnvalue "_ExtraLong"))) (`KismetStringLibrary.Conv_StringToName` (`KismetStringLibrary.Concat_StrStr` "CableLoc" (`KismetStringLibrary.Conv_IntToString` _returnvalue_2))) (`KismetStringLibrary.Conv_StringToName` (`KismetStringLibrary.Concat_StrStr` "CableLoc" (`KismetStringLibrary.Conv_IntToString` (+ _returnvalue_2 1)))) (select `bool` (and (> _numcablesspawned 7) (< _numcablesspawned 12)) :`true` "CableLocLong" :!type "Name") (select `bool` (or (== _numcablesspawned 9) (== _numcablesspawned 10)) :`true` "CableLocExtraLong" :!type "Name") null)
      (set `self.isSpawned` true)
      (set `self.NumCablesSpawned` (+ (`self.NumCablesSpawned`) 1)))))

(fn `UserConstructionScript`)