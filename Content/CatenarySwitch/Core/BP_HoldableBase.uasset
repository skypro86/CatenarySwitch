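; Base VR grippable object for the catenary switch game that players mount on a BP_Pole at a target position.
; Tick sphere-traces for the tagged pole, then attaches to its socket with a physics constraint.
; It compares Z or X against the pole's target, denying grip when correct and otherwise showing an outline outside Switch_Hard levels.
; A text render displays height, and a looping timer returns fallen objects to their start transform.
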(event `self.GrippableStaticMesh.OnDropped`
  (params (GrippingController :type "GripMotionControllerComponent Object Reference") (GripInformation :type "BPActorGripInformation Structure (by ref)") (bWasSocketed :type Boolean))
  (bind _grippablestaticmesh (`self.GrippableStaticMesh`))
  ; Disables Physics If snapped to pole
  (if (`self.IsSnapped`)
    (`PrimitiveComponent.SetSimulatePhysics` _grippablestaticmesh false)
    (bind _iscorrect (`self.CheckCorrectHeight` (`self.Socket Name`) _grippablestaticmesh))
    (if _iscorrect
      (`SceneComponent.SetVisibility` (`self.TextRender`) false false))))

(event `HeightCheck`
  (bind _grippablestaticmesh (`self.GrippableStaticMesh`))
  (bind (_returnvalue_x _returnvalue_y _returnvalue_z) (`KismetMathLibrary.BreakVector` (`SceneComponent.K2_GetComponentLocation` (`self.GrippableStaticMesh`))))
  ; Custom Event to resapwn the object if below a certain thershold
  (if (< _returnvalue_z 120.0)
    (`PrimitiveComponent.SetPhysicsLinearVelocity` _grippablestaticmesh (0.0 0.0 0.0) false "None")
    (`PrimitiveComponent.SetPhysicsAngularVelocityInRadians` _grippablestaticmesh (0.0 0.0 0.0) false "None")
    (`SceneComponent.K2_SetWorldLocation` _grippablestaticmesh (`self.Position`) false false)
    (`SceneComponent.K2_SetWorldRotation` _grippablestaticmesh (`self.Rotation`) false false)))

(event `self.ReceiveTick`
  (params (DeltaSeconds :type "Float (single-precision)"))
  (bind _grippablestaticmesh (`self.GrippableStaticMesh`))
  (bind _grippablestaticmesh_2 (`self.GrippableStaticMesh`))
  (bind _grippablestaticmesh_3 (`self.GrippableStaticMesh`))
  (bind _returnvalue (`SceneComponent.K2_GetComponentLocation` _grippablestaticmesh_2))
  (bind (_returnvalue_x _returnvalue_y _returnvalue_z) (`KismetMathLibrary.BreakVector` (`SceneComponent.K2_GetComponentLocation` (`self.GrippableStaticMesh`))))
  (`|ExecutionSequence`
    (:`then_0`
      ; Changes based on if the object is at the correct height or not
      (bind _iscorrect (`self.CheckCorrectHeight` (`self.Socket Name`) _grippablestaticmesh_2))
      (if _iscorrect
        (`GrippableStaticMeshComponent.SetDenyGripping` _grippablestaticmesh true)
        (bind _returnvalue_2 (`GameplayStatics.GetCurrentLevelName` true))
        (if (not (or (`KismetStringLibrary.EqualEqual_StrStr` _returnvalue_2 "Switch_Hard") (`KismetStringLibrary.EqualEqual_StrStr` _returnvalue_2 "Switch_Hard_TiltedLeft") (`KismetStringLibrary.EqualEqual_StrStr` _returnvalue_2 "Switch_Hard_TiltedRight")))
          (`MeshComponent.SetOverlayMaterial` _grippablestaticmesh_3 null))
        (else
          (`GrippableStaticMeshComponent.SetDenyGripping` _grippablestaticmesh false)
          (`SceneComponent.SetVisibility` (`self.TextRender`) true false)
          (bind _returnvalue_3 (`GameplayStatics.GetCurrentLevelName` true))
          (if (not (or (`KismetStringLibrary.EqualEqual_StrStr` _returnvalue_3 "Switch_Hard") (`KismetStringLibrary.EqualEqual_StrStr` _returnvalue_3 "Switch_Hard_TiltedLeft") (`KismetStringLibrary.EqualEqual_StrStr` _returnvalue_3 "Switch_Hard_TiltedRight")))
            (`MeshComponent.SetOverlayMaterial` _grippablestaticmesh_3 "/Game/CatenarySwitch/Art/Industrial/CatenarySwitch/M_Outline.M_Outline")))))
    (:`then_1`
      ; Checks for pole and snaps to pole if location is correct
      (bind (_outhit _returnvalue_4) (`KismetSystemLibrary.SphereTraceSingle` _returnvalue _returnvalue 30.0 "TraceTypeQuery3"))
      (if _returnvalue_4
        (bind (_bblockinghit _binitialoverlap _time _distance _location _impactpoint _normal _impactnormal _physmat _hitactor _hitcomponent) (`GameplayStatics.BreakHitResult` _outhit))
        (if (and (not (`self.IsSnapped`)) (`ActorComponent.ComponentHasTag` _hitcomponent (`self.Tag`)))
          (bind _asbp_pole (cast `/Game/CatenarySwitch/Art/Industrial/CatenarySwitch/Blueprints/BP_Pole` _hitactor))
          (set `self.Pole` _asbp_pole)
          (`SceneComponent.K2_AttachToComponent` _grippablestaticmesh_2 (`/Game/CatenarySwitch/Art/Industrial/CatenarySwitch/Blueprints/BP_Pole.Pole` (`self.Pole`)) (`self.Socket Name`) "SnapToTarget" "SnapToTarget" "SnapToTarget" true)
          (`PhysicsConstraintComponent.SetConstrainedComponents` (`self.PhysicsConstraint`) _grippablestaticmesh_2 "None" (`/Game/CatenarySwitch/Art/Industrial/CatenarySwitch/Blueprints/BP_Pole.Pole` (`self.Pole`)) "None")
          (set `self.IsSnapped` true)
          (`PrimitiveComponent.SetCollisionResponseToChannel` _grippablestaticmesh_2 "ECC_WorldStatic" "ECR_Ignore")
          (`PrimitiveComponent.SetEnableGravity` _grippablestaticmesh_2 false)
          (`PrimitiveComponent.SetCollisionObjectType` _grippablestaticmesh_2 "ECC_WorldStatic"))
        (else
          (set `self.IsSnapped` false))))
    (:`then_2`
      (`TextRenderComponent.K2_SetText` (`self.TextRender`) (`KismetTextLibrary.Conv_DoubleToText` (/ (- _returnvalue_z 145.0) 100.0) "HalfToEven" false true 1 324 0 2)))))

(event `self.ReceiveBeginPlay`
  (bind _grippablestaticmesh (`self.GrippableStaticMesh`))
  ; Sets Up Object inital Position Rotation and start Custom Even
  (set `self.Position` (`SceneComponent.K2_GetComponentLocation` _grippablestaticmesh))
  (set `self.Rotation` (`SceneComponent.K2_GetComponentRotation` _grippablestaticmesh))
  (`KismetSystemLibrary.K2_SetTimer` null "HeightCheck" 0.1 true))

(fn `AdvancedGripSettings`
  (returns (ReturnValue :type "BPAdvGripSettings Structure"))
  (return))

(fn `AllowsMultipleGrips`
  (returns (ReturnValue :type Boolean))
  (return false))

(fn `CheckCorrectHeight`
  (params (`Socket Name` :type Name) (GrippableStatciMesh :type "GrippableStaticMeshComponent Object Reference"))
  (returns (IsCorrect :type Boolean))
  (bind _returnvalue_x (`KismetMathLibrary.BreakVector` (`SceneComponent.K2_GetComponentLocation` GrippableStatciMesh)))
  (bind (_returnvalue_x_2 _returnvalue_y _returnvalue_z) (`KismetMathLibrary.BreakVector` (`SceneComponent.K2_GetComponentLocation` GrippableStatciMesh)))
  (bind _pole (`self.Pole`)
    (:`then`
      (bind (_value _returnvalue) (`BlueprintMapLibrary.Map_Find` (`/Game/CatenarySwitch/Art/Industrial/CatenarySwitch/Blueprints/BP_Pole.CorrectHeightCollection` _pole) `Socket Name`))
      (if _returnvalue
        (if (`self.IsVertical`)
          (bind (_returnvalue_x_3 _returnvalue_y_2 _returnvalue_z_2) (`KismetMathLibrary.BreakVector` (`SceneComponent.K2_GetComponentLocation` _value)))
          (return (`KismetMathLibrary.NearlyEqual_FloatFloat` _returnvalue_z_2 _returnvalue_z (`self.Error Tolerance`)))
          (else
            (bind _returnvalue_x_4 (`KismetMathLibrary.BreakVector` (`SceneComponent.K2_GetComponentLocation` _value)))
            (return (`KismetMathLibrary.NearlyEqual_FloatFloat` _returnvalue_x_4 _returnvalue_x (`self.Error Tolerance`)))))
        (else
          _)))
    (:`else`
      _))
  (return false))

(fn `ClosestGripSlotInRange`
  (params (WorldLocation :type "Vector Structure") (bSecondarySlot :type Boolean) (CallingController :type "GripMotionControllerComponent Object Reference") (OverridePrefix :type Name))
  (returns (bHadSlotInRange :type Boolean) (SlotWorldTransform :type "Transform Structure") (SlotName :type Name))
  (return false (struct) "None"))

(fn `DenyGripping`
  (params (GripInitiator :type "GripMotionControllerComponent Object Reference"))
  (returns (ReturnValue :type Boolean))
  (return false))

(fn `GetGripScripts`
  (returns (ArrayReference :type "Array of VRGripScriptBase Object Reference") (ReturnValue :type Boolean))
  (return _ false))

(fn `GetGripStiffnessAndDamping`
  (returns (GripStiffnessOut :type "Float (single-precision)") (GripDampingOut :type "Float (single-precision)"))
  (return 0.0 0.0))

(fn `GetPrimaryGripType`
  (params (bIsSlot :type Boolean))
  (returns (ReturnValue :type "EGripCollisionType Enum"))
  (return "InteractiveCollisionWithPhysics"))

(fn `GripBreakDistance`
  (returns (ReturnValue :type "Float (single-precision)"))
  (return 0.0))

(fn `GripLateUpdateSetting`
  (returns (ReturnValue :type "EGripLateUpdateSettings Enum"))
  (return "LateUpdatesAlwaysOn"))

(fn `GripMovementReplicationType`
  (returns (ReturnValue :type "EGripMovementReplicationSettings Enum"))
  (return "KeepOriginalMovement"))

(fn `IsHeld`
  (returns (HoldingControllers :type "Array of BPGripPair Structure") (bIsHeld :type Boolean))
  (return _ false))

(fn `RequestsSocketing`
  (returns (ParentToSocketTo :type "SceneComponent Object Reference") (OptionalSocketName :type Name) (RelativeTransform :type "Transform_NetQuantize Structure") (ReturnValue :type Boolean))
  (return null "None" (struct) false))

(fn `SecondaryGripType`
  (returns (ReturnValue :type "ESecondaryGripType Enum"))
  (return "SG_None"))

(fn `SimulateOnDrop`
  (returns (ReturnValue :type Boolean))
  (return false))

(fn `TeleportBehavior`
  (returns (ReturnValue :type "EGripInterfaceTeleportBehavior Enum"))
  (return "TeleportAllComponents"))

(fn `UserConstructionScript`)