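; BP_FinalCheck is a world-progression actor with a button that shows and hides its BPExplanations component.
; The component starts hidden at BeginPlay, and each press alternates its visibility through a FlipFlop, without propagating to children.
; The press handler immediately clears the button's state, so it acts as a momentary trigger rather than a latched switch.
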(event `self.ReceiveBeginPlay`
  (`SceneComponent.SetVisibility` (`self.BP_Explanations`) false false))

(event `self.ButtonComponent.ButtonPressed`
  (params (ButtonState :type Boolean))
  (if ButtonState
    (set `/Game/VRE/Grippables/Misc/Examples/Button/ButtonComponent.ButtonState` false (`self.ButtonComponent`))
    (`/Engine/EditorBlueprintResources/StandardMacros.FlipFlop`
      (:`A`
        (`SceneComponent.SetVisibility` (`self.BP_Explanations`) true false))
      (:`B`
        (`SceneComponent.SetVisibility` (`self.BP_Explanations`) false false)))))

(fn `UserConstructionScript`)