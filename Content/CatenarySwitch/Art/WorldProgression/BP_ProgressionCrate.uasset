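; BP_ProgressionCrate is a progression blocker that disappears once its associated catenary switch part is correctly placed.
; On Tick, BoxNum selects the switch box, cable protector or fixed switch, found via GetActorOfClass, and polls its CheckCorrectHeight against a named socket.
; When the check passes, the crate's five cube meshes are hidden and lose collision.
; An unconnected two-clamp check remains unused.
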(event `self.ReceiveTick`
  (params (DeltaSeconds :type "Float (single-precision)"))
  (switch `int` (`self.BoxNum`)
    (:`0`
      (bind _returnvalue (`GameplayStatics.GetActorOfClass` "/Game/CatenarySwitch/Art/Industrial/CatenarySwitch/Blueprints/BP_SwitchBox.BP_SwitchBox_C"))
      (bind _iscorrect (`/Game/CatenarySwitch/Core/BP_HoldableBase.CheckCorrectHeight` _returnvalue "Socket_SwitchBox" (`/Game/CatenarySwitch/Core/BP_HoldableBase.GrippableStaticMesh` _returnvalue)))
      (if _iscorrect
        (for _array_element (`|MakeArray` (`self.SM_Cube`) (`self.SM_Cube1`) (`self.SM_Cube2`) (`self.SM_Cube3`) (`self.SM_Cube4`)) :!label _label
          (`SceneComponent.SetVisibility` _array_element false false)
          (`PrimitiveComponent.SetCollisionEnabled` _array_element "NoCollision"))))
    (:`1`
      (bind _returnvalue_2 (`GameplayStatics.GetActorOfClass` "/Game/CatenarySwitch/Art/Industrial/CatenarySwitch/Blueprints/BP_MB_CableProtector2.BP_MB_CableProtector2_C"))
      (bind _iscorrect_2 (`/Game/CatenarySwitch/Core/BP_HoldableBase.CheckCorrectHeight` _returnvalue_2 "Socket_MB_CableProtector2" (`/Game/CatenarySwitch/Core/BP_HoldableBase.GrippableStaticMesh` _returnvalue_2)))
      (if _iscorrect_2
        (goto _label)))
    (:`2`
      (bind _returnvalue_3 (`GameplayStatics.GetActorOfClass` "/Game/CatenarySwitch/Art/Industrial/CatenarySwitch/Blueprints/BP_Switch_Fixed.BP_Switch_Fixed_C"))
      (bind _iscorrect_3 (`/Game/CatenarySwitch/Core/BP_HoldableBase.CheckCorrectHeight` _returnvalue_3 "Socket_Switch_Fixed" (`/Game/CatenarySwitch/Core/BP_HoldableBase.GrippableStaticMesh` _returnvalue_3)))
      (if _iscorrect_3
        (goto _label)))))

(fn `UserConstructionScript`)