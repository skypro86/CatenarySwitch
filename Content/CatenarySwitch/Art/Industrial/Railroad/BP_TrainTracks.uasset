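; BP_TrainTracks is a spline-driven actor that lays railroad track by repeating a mesh along an editable spline.
; The construction script divides the spline length by MeshSize and adds one spline mesh component with collision per whole segment, so any leftover length stays uncovered.
; Each segment takes its endpoints and tangents from the spline, with tangent length clamped to MeshSize to limit distortion.
; The event graph has no active logic.
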(fn `UserConstructionScript`
  (bind _mesh_size (`self.Mesh Size`))
  (bind _spline (`self.Spline`))
  (bind _spline_2 (`self.Spline`))
  (bind _returnvalue (`KismetMathLibrary.FTrunc` (/ (`SplineComponent.GetSplineLength` (`self.Spline`)) (`self.Mesh Size`))))
  (if (> _returnvalue 0)
    (for _index (range _returnvalue)
      (bind _returnvalue_2 (`AddComponent|NODE_AddSplineMeshComponent-0`))
      (bind _returnvalue_3 (* _index _mesh_size))
      (bind _returnvalue_4 (+ _returnvalue_3 _mesh_size))
      (`SplineMeshComponent.SetStartAndEnd` _returnvalue_2 (`SplineComponent.GetLocationAtDistanceAlongSpline` _spline_2 _returnvalue_3 "Local") (`KismetMathLibrary.ClampVectorSize` (`SplineComponent.GetTangentAtDistanceAlongSpline` _spline_2 _returnvalue_3 "Local") 0.0 _mesh_size) (`SplineComponent.GetLocationAtDistanceAlongSpline` _spline _returnvalue_4 "Local") (`KismetMathLibrary.ClampVectorSize` (`SplineComponent.GetTangentAtDistanceAlongSpline` _spline _returnvalue_4 "Local") 0.0 _mesh_size) true)
      (`PrimitiveComponent.SetCollisionEnabled` _returnvalue_2 "QueryAndPhysics")
      (`StaticMeshComponent.SetStaticMesh` _returnvalue_2 (`self.Mesh`)))))