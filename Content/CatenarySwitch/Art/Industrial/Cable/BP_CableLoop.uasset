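; Physics-simulated catenary cable that snaps onto sockets on power cables, switches, powerline holders and poles.
; Construction builds NumLinks constrained mesh links, a spline and spline mesh segments.
; Post-physics Tick sphere-traces at fixed links, attaching tagged hits in length-dependent order with targets chosen via LengthToCableMap, then refits the spline meshes to the links.
; The logic signalling BP_CableSpawner and freezing finished cables is disconnected.
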(event `self.ReceiveBeginPlay`
  (`self.SetTickGroup` "TG_PostPhysics"))

(event `self.ReceiveTick`
  (params (DeltaSeconds :type "Float (single-precision)"))
  (bind _spline (`self.Spline`))
  (bind _spline_2 (`self.Spline`))
  (bind _value (`BlueprintMapLibrary.Map_Find` (`self.LengthToCableMap`) (`self.NumLinks`)))
  (bind _value_2 (`BlueprintMapLibrary.Map_Find` (`self.LengthToCableMap`) (`self.NumLinks`)))
  (bind _output (`|GetArrayItem` (`self.Links`) 85))
  (bind _output_2 (`|GetArrayItem` (`self.Links`)))
  (bind _output_3 (`|GetArrayItem` (`self.Links`) 46))
  (bind _output_4 (`|GetArrayItem` (`self.Links`) 75))
  (bind _output_5 (`|GetArrayItem` (`self.Links`) 10))
  (bind _returnvalue (`SceneComponent.K2_GetComponentLocation` _output_2))
  (bind _returnvalue_2 (`SceneComponent.K2_GetComponentLocation` _output_3))
  (bind _returnvalue_3 (`SceneComponent.K2_GetComponentLocation` _output_5))
  (bind _returnvalue_4 (`SceneComponent.K2_GetComponentLocation` _output_4))
  (bind _returnvalue_5 (`SceneComponent.K2_GetComponentLocation` _output))
  (bind _output_6 (`|GetArrayItem` (`self.Links`) (- (`self.NumLinks`) 1)))
  (bind _returnvalue_6 (`SceneComponent.K2_GetComponentLocation` _output_6))
  (`|ExecutionSequence`
    (:`then_0`
      ; Checks if cable is ready to be snapped
      (if true
        (`|ExecutionSequence`
          (:`then_0`
            ; Snapping to first socket function
            (bind (_outhit _returnvalue_7) (`KismetSystemLibrary.SphereTraceSingle` _returnvalue _returnvalue 30.0 "TraceTypeQuery3"))
            (if _returnvalue_7
              (bind (_bblockinghit _binitialoverlap _time _distance _location _impactpoint _normal _impactnormal _physmat _hitactor _hitcomponent) (`GameplayStatics.BreakHitResult` _outhit))
              (if (and (not (`self.IsSnapped 1`)) (`ActorComponent.ComponentHasTag` _hitcomponent (`self.Tag 1`)))
                (switch `int` _value_2
                  (:`0`
                    (bind _asbp_power_cable (cast `/Game/CatenarySwitch/Art/Industrial/CatenarySwitch/Blueprints/BP_PowerCable` _hitactor)
                      (:`then`
                        (bind _output_get (set `self.PowerCable` _asbp_power_cable))
                        (bind _grippablestaticmesh (`/Game/CatenarySwitch/Core/BP_HoldableBase.GrippableStaticMesh` (stale _output_get_3)))
                        (bind _returnvalue_8 (select `int` _value_2 :`0` (`/Game/CatenarySwitch/Core/BP_HoldableBase.GrippableStaticMesh` _output_get) :`1` (`/Game/CatenarySwitch/Core/BP_HoldableBase.GrippableStaticMesh` (stale _output_get_2)) :`2` _grippablestaticmesh :`3` _grippablestaticmesh :!type "StaticMeshComponent Object Reference"))
                        (`SceneComponent.K2_AttachToComponent` _output_2 _returnvalue_8 (`self.Socket Name 1`) "SnapToTarget" "SnapToTarget" "SnapToTarget" true :!label _label)
                        (`PhysicsConstraintComponent.SetConstrainedComponents` (`self.PhysicsConstraint1`) _output_2 "None" _returnvalue_8 "None")
                        (set `self.IsSnapped 1` true)
                        (`PrimitiveComponent.SetCollisionResponseToChannel` _output_2 "ECC_WorldStatic" "ECR_Ignore")
                        (`PrimitiveComponent.SetEnableGravity` _output_2 false)
                        (`PrimitiveComponent.SetSimulatePhysics` _output_2 false))
                      (:`CastFailed`
                        (`KismetSystemLibrary.PrintString` "Cast Failed" :!label _label_2))))
                  (:`1`
                    (bind _asbp_switch_movable (cast `/Game/CatenarySwitch/Art/Industrial/CatenarySwitch/Blueprints/BP_Switch_Movable` _hitactor)
                      (:`then`
                        (bind _output_get_2 (set `self.MovableSwitch` _asbp_switch_movable))
                        (goto _label))
                      (:`CastFailed`
                        (goto _label_2))))
                  (:`2`
                    (bind _asbp_switch_fixed (cast `/Game/CatenarySwitch/Art/Industrial/CatenarySwitch/Blueprints/BP_Switch_Fixed` _hitactor :!label _label_3)
                      (:`then`
                        (bind _output_get_3 (set `self.FixedSwitch` _asbp_switch_fixed))
                        (goto _label))
                      (:`CastFailed`
                        (goto _label_2))))
                  (:`3`
                    (goto _label_3))))
              (else
                (set `self.IsSnapped 1` false))))
          (:`then_1`
            ; Snapping to second socket function
            (if (> (`self.NumLinks`) 40)
              (if (`self.IsSnapped 1`)
                (bind (_outhit_2 _returnvalue_9) (`KismetSystemLibrary.SphereTraceSingle` _returnvalue_3 _returnvalue_3 30.0 "TraceTypeQuery3"))
                (if _returnvalue_9
                  (bind (_bblockinghit_2 _binitialoverlap_2 _time_2 _distance_2 _location_2 _impactpoint_2 _normal_2 _impactnormal_2 _physmat_2 _hitactor_2 _hitcomponent_2) (`GameplayStatics.BreakHitResult` _outhit_2))
                  (if (and (not (`self.IsSnapped Long`)) (`ActorComponent.ComponentHasTag` _hitcomponent_2 (`self.Tag Long`)))
                    (bind _asbp_powerline_holder (cast `/Game/CatenarySwitch/Art/Industrial/CatenarySwitch/Blueprints/BP_Powerline_Holder` _hitactor_2))
                    (bind _output_get_4 (set `self.PowerLineHolder` _asbp_powerline_holder))
                    (bind _grippablestaticmesh_2 (`/Game/CatenarySwitch/Core/BP_HoldableBase.GrippableStaticMesh` _output_get_4))
                    (`SceneComponent.K2_AttachToComponent` _output_5 _grippablestaticmesh_2 (`self.Socket Name Long`) "SnapToTarget" "SnapToTarget" "SnapToTarget" true)
                    (`PhysicsConstraintComponent.SetConstrainedComponents` (`self.PhysicsConstraintLong`) _output_5 "None" _grippablestaticmesh_2 "None")
                    (set `self.IsSnapped Long` true)
                    (`PrimitiveComponent.SetCollisionResponseToChannel` _output_5 "ECC_WorldStatic" "ECR_Ignore")
                    (`PrimitiveComponent.SetEnableGravity` _output_5 false)
                    (`PrimitiveComponent.SetSimulatePhysics` _output_5 false))
                  (else
                    (set `self.IsSnapped Long` false))))))
          (:`then_2`
            ; Snapping to third socket function
            (if (> (`self.NumLinks`) 80)
              (if (`self.IsSnapped Long`)
                (bind (_outhit_3 _returnvalue_10) (`KismetSystemLibrary.SphereTraceSingle` _returnvalue_2 _returnvalue_2 30.0 "TraceTypeQuery3"))
                (if _returnvalue_10
                  (bind (_bblockinghit_3 _binitialoverlap_3 _time_3 _distance_3 _location_3 _impactpoint_3 _normal_3 _impactnormal_3 _physmat_3 _hitactor_3 _hitcomponent_3) (`GameplayStatics.BreakHitResult` _outhit_3))
                  (if (and (not (`self.IsSnapped ExtraLong`)) (`ActorComponent.ComponentHasTag` _hitcomponent_3 (`self.Tag ExtraLong`)))
                    (bind _asbp_pole (cast `/Game/CatenarySwitch/Art/Industrial/CatenarySwitch/Blueprints/BP_Pole` _hitactor_3))
                    (bind _output_get_5 (set `self.Pole` _asbp_pole))
                    (`SceneComponent.K2_AttachToComponent` _output_3 (`/Game/CatenarySwitch/Art/Industrial/CatenarySwitch/Blueprints/BP_Pole.Pole` _output_get_5) (`self.Socket Name ExtraLong`) "SnapToTarget" "SnapToTarget" "SnapToTarget" true)
                    (`PhysicsConstraintComponent.SetConstrainedComponents` (`self.PhysicsConstraintLong`) _output_3 "None" (`/Game/CatenarySwitch/Art/Industrial/CatenarySwitch/Blueprints/BP_Pole.Pole` (`self.Pole`)) "None")
                    (set `self.IsSnapped ExtraLong` true)
                    (`PrimitiveComponent.SetCollisionResponseToChannel` _output_3 "ECC_WorldStatic" "ECR_Ignore")
                    (`PrimitiveComponent.SetEnableGravity` _output_3 false)
                    (`PrimitiveComponent.SetSimulatePhysics` _output_3 false))
                  (else
                    (set `self.IsSnapped ExtraLong` false))))))
          (:`then_3`
            ; Snapping to last socket function
            (if (> (`self.NumLinks`) 80)
              (if (`self.IsSnapped ExtraLong`)
                (if (`self.IsSnapped 1`) :!label _label_4
                  (bind (_outhit_4 _returnvalue_11) (`KismetSystemLibrary.SphereTraceSingle` _returnvalue_6 _returnvalue_6 30.0 "TraceTypeQuery3"))
                  (if _returnvalue_11
                    (bind (_bblockinghit_4 _binitialoverlap_4 _time_4 _distance_4 _location_4 _impactpoint_4 _normal_4 _impactnormal_4 _physmat_4 _hitactor_4 _hitcomponent_4) (`GameplayStatics.BreakHitResult` _outhit_4))
                    (if (and (not (`self.IsSnapped 2`)) (`ActorComponent.ComponentHasTag` _hitcomponent_4 (`self.Tag 2`)))
                      (switch `int` _value
                        (:`0`
                          (bind _asbp_switch_fixed_2 (cast `/Game/CatenarySwitch/Art/Industrial/CatenarySwitch/Blueprints/BP_Switch_Fixed` _hitactor_4 :!label _label_5))
                          (bind _output_get_6 (set `self.FixedSwitch` _asbp_switch_fixed_2)))
                        (:`1`
                          (goto _label_5))
                        (:`2`
                          (bind _asbp_pole_2 (cast `/Game/CatenarySwitch/Art/Industrial/CatenarySwitch/Blueprints/BP_Pole` _hitactor_4 :!label _label_6))
                          (bind _output_get_7 (set `self.Pole` _asbp_pole_2)))
                        (:`3`
                          (goto _label_6)))
                      (bind _grippablestaticmesh_3 (`/Game/CatenarySwitch/Core/BP_HoldableBase.GrippableStaticMesh` _output_get_6))
                      (bind _pole (`/Game/CatenarySwitch/Art/Industrial/CatenarySwitch/Blueprints/BP_Pole.Pole` _output_get_7))
                      (bind _returnvalue_12 (select `int` _value :`0` _grippablestaticmesh_3 :`1` _grippablestaticmesh_3 :`2` _pole :`3` _pole :!type "StaticMeshComponent Object Reference"))
                      (`SceneComponent.K2_AttachToComponent` _output_6 _returnvalue_12 (`self.Socket Name 2`) "SnapToTarget" "SnapToTarget" "SnapToTarget" true)
                      (`PhysicsConstraintComponent.SetConstrainedComponents` (`self.PhysicsConstraint2`) _output_6 "None" _returnvalue_12 "None")
                      (set `self.IsSnapped 2` true)
                      (`PrimitiveComponent.SetCollisionResponseToChannel` _output_6 "ECC_WorldStatic" "ECR_Ignore")
                      (`PrimitiveComponent.SetEnableGravity` _output_6 false)
                      (`PrimitiveComponent.SetSimulatePhysics` _output_6 false))
                    (else
                      (set `self.IsSnapped 2` false)))))
              (else
                (goto _label_4))))
          (:`then_4`
            ; Snapping to loop sockets function
            (if (> (`self.NumLinks`) 80)
              (if (`self.IsSnapped ExtraLong`)
                (bind (_outhit_5 _returnvalue_13) (`KismetSystemLibrary.SphereTraceSingle` :`Start` _returnvalue_4 :`End` _returnvalue_4 :`Radius` 15.0 :`TraceChannel` "TraceTypeQuery3" :`DrawDebugType` "ForOneFrame"))
                (if _returnvalue_13
                  (bind (_bblockinghit_5 _binitialoverlap_5 _time_5 _distance_5 _location_5 _impactpoint_5 _normal_5 _impactnormal_5 _physmat_5 _hitactor_5 _hitcomponent_5) (`GameplayStatics.BreakHitResult` _outhit_5))
                  (if (and (not (`self.IsSnapped Loop1`)) (`ActorComponent.ComponentHasTag` _hitcomponent_5 (`self.Tag Loop1`)))
                    (bind _asbp_pole_3 (cast `/Game/CatenarySwitch/Art/Industrial/CatenarySwitch/Blueprints/BP_Pole` _hitactor_5))
                    (bind _output_get_8 (set `self.Pole` _asbp_pole_3))
                    (`SceneComponent.K2_AttachToComponent` _output_4 (`/Game/CatenarySwitch/Art/Industrial/CatenarySwitch/Blueprints/BP_Pole.Pole` _output_get_8) (`self.Socket Name Loop1`) "SnapToTarget" "SnapToTarget" "SnapToTarget" true)
                    (`PhysicsConstraintComponent.SetConstrainedComponents` (`self.PhysicsConstraintLoop1`) _output_4 "None" (`/Game/CatenarySwitch/Art/Industrial/CatenarySwitch/Blueprints/BP_Pole.Pole` (`self.Pole`)) "None")
                    (set `self.IsSnapped Loop1` true))
                  (else
                    (set `self.IsSnapped Loop1` false))))))
          (:`then_5`
            (if (> (`self.NumLinks`) 80)
              (if (`self.IsSnapped ExtraLong`)
                (bind (_outhit_6 _returnvalue_14) (`KismetSystemLibrary.SphereTraceSingle` :`Start` _returnvalue_5 :`End` _returnvalue_5 :`Radius` 15.0 :`TraceChannel` "TraceTypeQuery3" :`DrawDebugType` "ForOneFrame"))
                (if _returnvalue_14
                  (bind (_bblockinghit_6 _binitialoverlap_6 _time_6 _distance_6 _location_6 _impactpoint_6 _normal_6 _impactnormal_6 _physmat_6 _hitactor_6 _hitcomponent_6) (`GameplayStatics.BreakHitResult` _outhit_6))
                  (if (and (not (`self.IsSnapped Loop2`)) (`ActorComponent.ComponentHasTag` _hitcomponent_6 (`self.Tag Loop2`)))
                    (bind _asbp_pole_4 (cast `/Game/CatenarySwitch/Art/Industrial/CatenarySwitch/Blueprints/BP_Pole` _hitactor_6))
                    (bind _output_get_9 (set `self.Pole` _asbp_pole_4))
                    (`SceneComponent.K2_AttachToComponent` _output (`/Game/CatenarySwitch/Art/Industrial/CatenarySwitch/Blueprints/BP_Pole.Pole` _output_get_9) (`self.Socket Name Loop2`) "SnapToTarget" "SnapToTarget" "SnapToTarget" true)
                    (`PhysicsConstraintComponent.SetConstrainedComponents` (`self.PhysicsConstraintLoop2`) _output "None" (`/Game/CatenarySwitch/Art/Industrial/CatenarySwitch/Blueprints/BP_Pole.Pole` (`self.Pole`)) "None")
                    (set `self.IsSnapped Loop2` true))
                  (else
                    (set `self.IsSnapped Loop2` false)))))))))
    (:`then_1`
      ; Cable Updates
      (`|ExecutionSequence`
        (:`then_0`
          (for (_array_element _array_index) (`self.Links`)
            (`SplineComponent.SetLocationAtSplinePoint` (`self.Spline`) _array_index (`SceneComponent.K2_GetComponentLocation` _array_element) "World" true)))
        (:`then_1`
          (for (_array_element_2 _array_index_2) (`self.SplineMeshSegments`)
            (bind _returnvalue_15 (* _array_index_2 (`self.MeshLength`)))
            (bind _returnvalue_16 (* (+ _array_index_2 1) (`self.MeshLength`)))
            (`SplineMeshComponent.SetStartAndEnd` _array_element_2 (`SplineComponent.GetLocationAtDistanceAlongSpline` _spline _returnvalue_15 "Local") (`SplineComponent.GetTangentAtDistanceAlongSpline` _spline _returnvalue_15 "Local") (`SplineComponent.GetLocationAtDistanceAlongSpline` _spline_2 _returnvalue_16 "Local") (`SplineComponent.GetTangentAtDistanceAlongSpline` _spline_2 _returnvalue_16 "Local") true)))))
    (:`then_2`)))

(fn `CheckCorrectHeight`
  (params (`Socket Name` :type Name) (GrippableStatciMesh :type "StaticMeshComponent Object Reference"))
  (returns (IsCorrect :type Boolean))
  (bind (_returnvalue_x _returnvalue_y _returnvalue_z) (`KismetMathLibrary.BreakVector` (`SceneComponent.K2_GetComponentLocation` GrippableStatciMesh)))
  (bind _pole (`self.Pole`)
    (:`then`
      (bind (_value _returnvalue) (`BlueprintMapLibrary.Map_Find` (`/Game/CatenarySwitch/Art/Industrial/CatenarySwitch/Blueprints/BP_Pole.CorrectHeightCollection` _pole) `Socket Name`))
      (if _returnvalue
        (bind (_returnvalue_x_2 _returnvalue_y_2 _returnvalue_z_2) (`KismetMathLibrary.BreakVector` (`SceneComponent.K2_GetComponentLocation` _value)))
        (return (`KismetMathLibrary.NearlyEqual_FloatFloat` _returnvalue_z_2 _returnvalue_z (`self.Error Tolerance`)))
        (else
          _)))
    (:`else`
      _))
  (return false))

(fn `FirstSocketSelector`
  (returns (ReturnValue :type "GrippableStaticMeshComponent Object Reference"))
  (bind _returnvalue (`GameplayStatics.GetActorOfClass` "/Game/CatenarySwitch/Core/BP_CableSpawner.BP_CableSpawner_C"))
  (return (select `int` (/ (`/Game/CatenarySwitch/Core/BP_CableSpawner.NumCablesSpawned` _returnvalue) 4) :`0` (`/Game/CatenarySwitch/Core/BP_HoldableBase.GrippableStaticMesh` (`self.PowerCable`)) :`1` (`/Game/CatenarySwitch/Core/BP_HoldableBase.GrippableStaticMesh` (`self.MovableSwitch`)) :`2` (`/Game/CatenarySwitch/Core/BP_HoldableBase.GrippableStaticMesh` (`self.FixedSwitch`)))))

(fn `LastSocketSelector`
  (returns (ReturnValue :type "GrippableStaticMeshComponent Object Reference"))
  (bind _numlinks (`self.NumLinks`))
  (if (< _numlinks 20)
    (return (`/Game/CatenarySwitch/Core/BP_HoldableBase.GrippableStaticMesh` (`self.FixedSwitch`)))
    (else
      (return (select `bool` (== _numlinks 45) :`false` (`/Game/CatenarySwitch/Core/BP_HoldableBase.GrippableStaticMesh` (`self.Clamp`)) :`true` (`/Game/CatenarySwitch/Core/BP_HoldableBase.GrippableStaticMesh` (`self.Clamp_ContactWire`)))))))

(fn `ObjectSelecetSocket_1`
  (params (NewParam :type "Object Object Reference"))
  (returns (ReturnValue :type "GrippableStaticMeshComponent Object Reference"))
  (bind (_key _value) (`BlueprintMapLibrary.Map_GetKeyValueByIndex` (`self.LengthToCableMap`) (`self.NumLinks`)))
  (switch `int` _value
    (:`0`
      (bind _asbp_power_cable (cast `/Game/CatenarySwitch/Art/Industrial/CatenarySwitch/Blueprints/BP_PowerCable` NewParam)
        (:`then`
          (bind _output_get (set `self.PowerCable` _asbp_power_cable))
          (bind _grippablestaticmesh (`/Game/CatenarySwitch/Core/BP_HoldableBase.GrippableStaticMesh` (stale _output_get_3)))
          (return (select `int` _value :`0` (`/Game/CatenarySwitch/Core/BP_HoldableBase.GrippableStaticMesh` _output_get) :`1` (`/Game/CatenarySwitch/Core/BP_HoldableBase.GrippableStaticMesh` (stale _output_get_2)) :`2` _grippablestaticmesh :`3` _grippablestaticmesh)))
        (:`CastFailed`
          _)))
    (:`1`
      (bind _asbp_switch_movable (cast `/Game/CatenarySwitch/Art/Industrial/CatenarySwitch/Blueprints/BP_Switch_Movable` NewParam)
        (:`then`
          (bind _output_get_2 (set `self.MovableSwitch` _asbp_switch_movable))
          (return (select `int` _value :`0` (`/Game/CatenarySwitch/Core/BP_HoldableBase.GrippableStaticMesh` _output_get) :`1` (`/Game/CatenarySwitch/Core/BP_HoldableBase.GrippableStaticMesh` _output_get_2) :`2` _grippablestaticmesh :`3` _grippablestaticmesh)))
        (:`CastFailed`
          _)))
    (:`2`
      (bind _asbp_switch_fixed (cast `/Game/CatenarySwitch/Art/Industrial/CatenarySwitch/Blueprints/BP_Switch_Fixed` NewParam :!label _label)
        (:`then`
          (bind _output_get_3 (set `self.FixedSwitch` _asbp_switch_fixed))
          (return (select `int` _value :`0` (`/Game/CatenarySwitch/Core/BP_HoldableBase.GrippableStaticMesh` _output_get) :`1` (`/Game/CatenarySwitch/Core/BP_HoldableBase.GrippableStaticMesh` _output_get_2) :`2` _grippablestaticmesh :`3` _grippablestaticmesh)))
        (:`CastFailed`
          _)))
    (:`3`
      (goto _label)))
  (`KismetSystemLibrary.PrintString` "Cast failed"))

(fn `SnappingToSocket`
  (params (SocketPosition :type Integer)))

(fn `UserConstructionScript`
  (bind _links (`self.Links`))
  (for _index (range (`self.NumLinks`))
    (`|ExecutionSequence`
      (:`then_0`
        (bind _returnvalue (`AddComponent|NODE_AddStaticMeshComponent-0`))
        (`PrimitiveComponent.SetSimulatePhysics` _returnvalue true)
        (`SceneComponent.K2_AttachToComponent` _returnvalue (`self.Spline`) "None" "KeepWorld" "KeepWorld" "KeepWorld" false)
        (`SceneComponent.K2_SetRelativeLocation` _returnvalue (`KismetMathLibrary.MakeVector` (`KismetMathLibrary.Conv_IntToDouble` (* _index (`self.MeshLength`)))) false false)
        (`KismetArrayLibrary.Array_Add` (`self.Links`) _returnvalue))
      (:`then_1`
        (if (> _index 0)
          (bind _returnvalue_2 (`AddComponent|NODE_AddPhysicsConstraintComponent-0`))
          (`SceneComponent.K2_SetRelativeLocation` _returnvalue_2 (`KismetMathLibrary.MakeVector` (`KismetMathLibrary.Conv_IntToDouble` (* _index (`self.MeshLength`)))) false false)
          (`PhysicsConstraintComponent.SetConstrainedComponents` _returnvalue_2 (`|GetArrayItem` _links (- _index 1)) "None" (`|GetArrayItem` _links _index) "None")
          (`SceneComponent.K2_AttachToComponent` _returnvalue_2 (`self.RootComponent`) "None" "KeepWorld" "KeepWorld" "KeepWorld" false)
          (`KismetArrayLibrary.Array_Add` (`self.Constraints`) _returnvalue_2)))))
  (`|ExecutionSequence`
    (:`then_0`
      (`SplineComponent.ClearSplinePoints` (`self.Spline`) true)
      (for _array_element (`self.Links`)
        (`SplineComponent.AddSplinePoint` (`self.Spline`) (`SceneComponent.K2_GetComponentLocation` _array_element) "World" true)))
    (:`then_1`
      (for _ (`self.Links`)
        (bind _returnvalue_3 (`AddComponent|NODE_AddSplineMeshComponent-0`))
        (`SceneComponent.K2_AttachToComponent` _returnvalue_3 (`self.Spline`) "None" "KeepRelative" "KeepRelative" "KeepRelative" false)
        (`KismetArrayLibrary.Array_Add` (`self.SplineMeshSegments`) _returnvalue_3)))))