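; Tutorial physics cable whose two ends snap to sockets on BP_ProgressionCable.
; The construction script builds a chain of simulated mesh links joined by physics constraints, with a spline and spline meshes over them.
; Each Tick, sphere traces and pole-hit checks attach and freeze the end links, while the spline and meshes follow the chain.
; When both ends are snapped, it increments CablesPlaced once; the switch height check is disconnected.
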(event `self.ReceiveTick`
  (params (DeltaSeconds :type "Float (single-precision)"))
  (bind _spline (`self.Spline`))
  (bind _spline_2 (`self.Spline`))
  (bind _output (`|GetArrayItem` (`self.Links`)))
  (bind _returnvalue (`SceneComponent.K2_GetComponentLocation` (`|GetArrayItem` (`self.Links`))))
  (bind _output_2 (`|GetArrayItem` (`self.Links`) (- (`self.NumLinks`) 1)))
  (bind _returnvalue_2 (`SceneComponent.K2_GetComponentLocation` (`|GetArrayItem` (`self.Links`) (- (`self.NumLinks`) 1))))
  (`|ExecutionSequence`
    (:`then_0`
      ; Checks if prerequisits are placed at correct height
      (`|ExecutionSequence`
        (:`then_0`
          ; Snapping to first socket function
          (bind (_outhit _returnvalue_3) (`KismetSystemLibrary.SphereTraceSingle` _returnvalue _returnvalue 30.0 "TraceTypeQuery3"))
          (if _returnvalue_3
            (bind (_bblockinghit _binitialoverlap _time _distance _location _impactpoint _normal _impactnormal _physmat _hitactor _hitcomponent) (`GameplayStatics.BreakHitResult` _outhit))
            (if (and (not (`self.IsSnapped 1`)) (`ActorComponent.ComponentHasTag` _hitcomponent (`self.Tag 1`)))
              (bind _asbp_progression_cable (cast `/Game/CatenarySwitch/Art/WorldProgression/BP_ProgressionCable` _hitactor))
              (bind _output_get (set `self.CableTutorial` _asbp_progression_cable))
              (`SceneComponent.K2_AttachToComponent` _output (`/Game/CatenarySwitch/Art/WorldProgression/BP_ProgressionCable.Cable_Tutorial` _output_get) (`self.Socket Name 1`) "SnapToTarget" "SnapToTarget" "SnapToTarget" true)
              (`PhysicsConstraintComponent.SetConstrainedComponents` (`self.PhysicsConstraint1`) _output "None" (`/Game/CatenarySwitch/Art/WorldProgression/BP_ProgressionCable.Cable_Tutorial` (`self.CableTutorial`)) "None")
              (set `self.IsSnapped 1` true)
              (`PrimitiveComponent.SetCollisionResponseToChannel` _output "ECC_WorldStatic" "ECR_Ignore")
              (`PrimitiveComponent.SetEnableGravity` _output false)
              (`PrimitiveComponent.SetSimulatePhysics` _output false))
            (else
              (set `self.IsSnapped 1` false))))
        (:`then_1`
          ; Snapping to last socket function
          (bind (_outhit_2 _returnvalue_4) (`KismetSystemLibrary.SphereTraceSingle` _returnvalue_2 _returnvalue_2 30.0 "TraceTypeQuery3"))
          (if _returnvalue_4
            (bind (_bblockinghit_2 _binitialoverlap_2 _time_2 _distance_2 _location_2 _impactpoint_2 _normal_2 _impactnormal_2 _physmat_2 _hitactor_2 _hitcomponent_2) (`GameplayStatics.BreakHitResult` _outhit_2))
            (if (and (not (`self.IsSnapped 2`)) (`ActorComponent.ComponentHasTag` _hitcomponent_2 (`self.Tag 2`)))
              (bind _asbp_progression_cable_2 (cast `/Game/CatenarySwitch/Art/WorldProgression/BP_ProgressionCable` _hitactor_2))
              (bind _output_get_2 (set `self.CableTutorial` _asbp_progression_cable_2))
              (`SceneComponent.K2_AttachToComponent` _output_2 (`/Game/CatenarySwitch/Art/WorldProgression/BP_ProgressionCable.Cable_Tutorial` _output_get_2) (`self.Socket Name 2`) "SnapToTarget" "SnapToTarget" "SnapToTarget" true)
              (`PhysicsConstraintComponent.SetConstrainedComponents` (`self.PhysicsConstraint2`) _output_2 "None" (`/Game/CatenarySwitch/Art/WorldProgression/BP_ProgressionCable.Cable_Tutorial` (`self.CableTutorial`)) "None")
              (set `self.IsSnapped 2` true)
              (`PrimitiveComponent.SetCollisionResponseToChannel` _output_2 "ECC_WorldStatic" "ECR_Ignore")
              (`PrimitiveComponent.SetEnableGravity` _output_2 false)
              (`PrimitiveComponent.SetSimulatePhysics` _output_2 false))
            (else
              (set `self.IsSnapped 2` false))))))
    (:`then_1`
      ; Cable Updates
      (`|ExecutionSequence`
        (:`then_0`
          (for (_array_element _array_index) (`self.Links`)
            (`SplineComponent.SetLocationAtSplinePoint` (`self.Spline`) _array_index (`SceneComponent.K2_GetComponentLocation` _array_element) "World" true)))
        (:`then_1`
          (for (_array_element_2 _array_index_2) (`self.SplineMeshSegments`)
            (bind _returnvalue_5 (* _array_index_2 (`self.MeshLength`)))
            (bind _returnvalue_6 (* (+ _array_index_2 1) (`self.MeshLength`)))
            (`SplineMeshComponent.SetStartAndEnd` _array_element_2 (`SplineComponent.GetLocationAtDistanceAlongSpline` _spline _returnvalue_5 "Local") (`SplineComponent.GetTangentAtDistanceAlongSpline` _spline _returnvalue_5 "Local") (`SplineComponent.GetLocationAtDistanceAlongSpline` _spline_2 _returnvalue_6 "Local") (`SplineComponent.GetTangentAtDistanceAlongSpline` _spline_2 _returnvalue_6 "Local") true)))))
    (:`then_2`
      ; Checks if cable is snapped
      (if (and (`self.IsSnapped 1`) (`self.IsSnapped 2`))
        (`/Engine/EditorBlueprintResources/StandardMacros.DoOnce` false
          (:`Completed`
            (bind _returnvalue_7 (`GameplayStatics.GetActorOfClass` "/Game/CatenarySwitch/Art/WorldProgression/BP_ProgressionCable.BP_ProgressionCable_C"))
            (set `/Game/CatenarySwitch/Art/WorldProgression/BP_ProgressionCable.CablesPlaced` (+ (`/Game/CatenarySwitch/Art/WorldProgression/BP_ProgressionCable.CablesPlaced` _returnvalue_7) 1) _returnvalue_7)))))))

(fn `UserConstructionScript`
  (bind _links (`self.Links`))
  (for _index (range (`self.NumLinks`))
    (`|ExecutionSequence`
      (:`then_0`
        (bind _returnvalue (`AddComponent|NODE_AddStaticMeshComponent-0`))
        (`PrimitiveComponent.SetSimulatePhysics` _returnvalue true)
        (`SceneComponent.K2_AttachToComponent` _returnvalue (`self.Spline`) "None" "KeepWorld" "KeepWorld" "KeepWorld" false)
        (`SceneComponent.K2_SetRelativeLocation` _returnvalue (`KismetMathLibrary.MakeVector` (`KismetMathLibrary.Conv_IntToDouble` (* _index (`self.MeshLength`)))) false false)
        (`KismetArrayLibrary.Array_Add` (`self.Links`) _returnvalue))
      (:`then_1`
        (if (> _index 0)
          (bind _returnvalue_2 (`AddComponent|NODE_AddPhysicsConstraintComponent-0`))
          (`SceneComponent.K2_SetRelativeLocation` _returnvalue_2 (`KismetMathLibrary.MakeVector` (`KismetMathLibrary.Conv_IntToDouble` (* _index (`self.MeshLength`)))) false false)
          (`PhysicsConstraintComponent.SetConstrainedComponents` _returnvalue_2 (`|GetArrayItem` _links (- _index 1)) "None" (`|GetArrayItem` _links _index) "None")
          (`SceneComponent.K2_AttachToComponent` _returnvalue_2 (`self.RootComponent`) "None" "KeepWorld" "KeepWorld" "KeepWorld" false)
          (`KismetArrayLibrary.Array_Add` (`self.Constraints`) _returnvalue_2)))))
  (`|ExecutionSequence`
    (:`then_0`
      (`SplineComponent.ClearSplinePoints` (`self.Spline`) true)
      (for _array_element (`self.Links`)
        (`SplineComponent.AddSplinePoint` (`self.Spline`) (`SceneComponent.K2_GetComponentLocation` _array_element) "World" true)))
    (:`then_1`
      (for _ (`self.Links`)
        (bind _returnvalue_3 (`AddComponent|NODE_AddSplineMeshComponent-0`))
        (`SceneComponent.K2_AttachToComponent` _returnvalue_3 (`self.Spline`) "None" "KeepRelative" "KeepRelative" "KeepRelative" false)
        (`KismetArrayLibrary.Array_Add` (`self.SplineMeshSegments`) _returnvalue_3)))))