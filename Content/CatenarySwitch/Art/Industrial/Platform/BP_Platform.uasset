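; VR lift platform that carries the player up, down and horizontally while their body is inside its trigger box.
; Held-object inputs or PageUp/PageDown scrub a height timeline on Base; right thumbstick or N/M drive a Control timeline through the Normal Play Logic macro.
; A barrier appears once Base reaches a height threshold, and the button resets both timelines.
; In tutorial levels, the lift stays hidden until BP_SwitchBox passes its height check.
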(event `self.ReceiveTick`
  (params (DeltaSeconds :type "Float (single-precision)"))
  (bind _barrier (`self.Barrier`))
  (bind _buttonpedestal (`self.ButtonPedestal`))
  (bind _base (`self.Base`))
  (bind (_returnvalue_x _returnvalue_y _returnvalue_z) (`KismetMathLibrary.BreakVector` (`SceneComponent.K2_GetComponentLocation` (`self.Base`))))
  ; Barrier Spawner
  (`|ExecutionSequence`
    (:`then_0`
      ; Spawn Lifts
      (bind _returnvalue (`GameplayStatics.GetCurrentLevelName` true))
      (if (or (`KismetStringLibrary.EqualEqual_StrStr` _returnvalue "Switch_Easy") (`KismetStringLibrary.EqualEqual_StrStr` _returnvalue "Switch_EasyRight") (`KismetStringLibrary.EqualEqual_StrStr` _returnvalue "Switch_EasyLeft"))
        (bind _returnvalue_2 (`GameplayStatics.GetActorOfClass` "/Game/CatenarySwitch/Art/Industrial/CatenarySwitch/Blueprints/BP_SwitchBox.BP_SwitchBox_C"))
        (bind _iscorrect (`/Game/CatenarySwitch/Core/BP_HoldableBase.CheckCorrectHeight` _returnvalue_2 "Socket_SwitchBox" (`/Game/CatenarySwitch/Core/BP_HoldableBase.GrippableStaticMesh` _returnvalue_2)))
        (if _iscorrect
          (`SceneComponent.SetVisibility` _buttonpedestal true true)
          (`PrimitiveComponent.SetCollisionEnabled` _buttonpedestal "QueryAndPhysics")
          (`SceneComponent.SetVisibility` _base true false)
          (`PrimitiveComponent.SetCollisionEnabled` _base "QueryAndPhysics"))))
    (:`then_1`
      (if (>= _returnvalue_z -20.0)
        (if (not (`self.IsBlocked`))
          (`SceneComponent.SetVisibility` _barrier true false)
          (`PrimitiveComponent.SetCollisionEnabled` _barrier "QueryAndPhysics")
          (set `self.IsBlocked` true))
        (elif (`self.IsBlocked`)
          (`SceneComponent.SetVisibility` _barrier false false)
          (`PrimitiveComponent.SetCollisionEnabled` _barrier "NoCollision")
          (set `self.IsBlocked` false))))))

(event `Key|PageUp`
  (params (Key :type "Key Structure"))
  (bind (_startpos_x _startpos_y _startpos_z) (`KismetMathLibrary.BreakVector` (`self.StartPos`)))
  (bind (_endpos_x _endpos_y _endpos_z) (`KismetMathLibrary.BreakVector` (`self.EndPos`)))
  ; Up/Down Movement
  (:`Pressed`
    (if (`self.IsPlayerInside`) :!label _label
      (bind (_direction _newtrack_0) (`Timeline|MovementTimeline` :`NewTime` (`self.Duration`) :!label _label_2)
        (:`Update`
          (`SceneComponent.K2_SetRelativeLocation` (`self.Base`) (`KismetMathLibrary.VLerp` (`KismetMathLibrary.MakeVector` 0.0 0.0 _startpos_z) (`KismetMathLibrary.MakeVector` 0.0 0.0 _endpos_z) _newtrack_0) false false)))))
  (:`Released`
    (goto _label_2 :!via `Stop`)))

(event `EnhancedInput|/Game/VRE/Input/Actions/UseHeldObjectRight`
  (params (ActionValue :type Boolean) (ElapsedSeconds :type "Float (double-precision)") (TriggeredSeconds :type "Float (double-precision)") (InputAction :type "InputAction Object Reference" :default "/Game/VRE/Input/Actions/UseHeldObjectRight.UseHeldObjectRight"))
  ; Up/Down Movement
  (:`Triggered`
    (goto _label))
  (:`Completed`
    (goto _label_2 :!via `Stop`)))

(event `EnhancedInput|/Game/VRE/Input/Actions/UseHeldObjectLeft`
  (params (ActionValue :type Boolean) (ElapsedSeconds :type "Float (double-precision)") (TriggeredSeconds :type "Float (double-precision)") (InputAction :type "InputAction Object Reference" :default "/Game/VRE/Input/Actions/UseHeldObjectLeft.UseHeldObjectLeft"))
  ; Up/Down Movement
  (:`Triggered`
    (if (`self.IsPlayerInside`) :!label _label_3
      (goto _label_2 :!via `Reverse`)))
  (:`Completed`
    (goto _label_2 :!via `Stop`)))

(event `Key|PageDown`
  (params (Key :type "Key Structure"))
  ; Up/Down Movement
  (:`Pressed`
    (goto _label_3))
  (:`Released`
    (goto _label_2 :!via `Stop`)))

(event `self.ButtonComponent.ButtonPressed`
  (params (ButtonState :type Boolean))
  (bind _endpos_x (`KismetMathLibrary.BreakVector` (`self.EndPos`)))
  (bind _startpos_x (`KismetMathLibrary.BreakVector` (`self.StartPos`)))
  ; Reset
  (if ButtonState
    (set `/Game/VRE/Grippables/Misc/Examples/Button/ButtonComponent.ButtonState` false (`self.ButtonComponent`))
    (`|ExecutionSequence` :!label _label_4
      (:`then_0`
        (goto _label_2 :!via `PlayFromStart`))
      (:`then_1`
        (goto _label_2 :!via `Stop`))
      (:`then_2`
        ; Normal Movement
        (bind (_direction _newtrack_0) (`Timeline|Timeline` :`NewTime` (`self.Duration`) :!via `PlayFromStart` :!label _label_5)
          (:`Update`
            (`SceneComponent.K2_SetRelativeLocation` (`self.Control`) (`KismetMathLibrary.VLerp` (`KismetMathLibrary.MakeVector` _startpos_x) (`KismetMathLibrary.MakeVector` _endpos_x) _newtrack_0) false false))))
      (:`then_3`
        (goto _label_5 :!via `Stop`)))))

(event `self.ReceiveBeginPlay`
  (bind _base (`self.Base`))
  (bind _buttonpedestal (`self.ButtonPedestal`))
  ; Position Setup
  (bind _output_get (set `self.StartPos` (`SceneComponent.RelativeLocation` (`self.Base`))))
  (set `self.EndPos` (+ _output_get (`KismetMathLibrary.MakeVector` (`self.ForwardOffSet`) 0.0 (`self.UpOffSet`))))
  (`|ExecutionSequence`
    (:`then_0`
      (goto _label_4))
    (:`then_1`
      ; Makes Lift Invisible
      (bind _returnvalue (`GameplayStatics.GetCurrentLevelName` true))
      (if (or (`KismetStringLibrary.EqualEqual_StrStr` _returnvalue "Switch_Easy") (`KismetStringLibrary.EqualEqual_StrStr` _returnvalue "Switch_EasyRight") (`KismetStringLibrary.EqualEqual_StrStr` _returnvalue "Switch_EasyLeft"))
        (`SceneComponent.SetVisibility` _buttonpedestal false true)
        (`PrimitiveComponent.SetCollisionEnabled` _buttonpedestal "NoCollision")
        (`SceneComponent.SetVisibility` _base false false)
        (`PrimitiveComponent.SetCollisionEnabled` _base "NoCollision")))))

(event `Key|N`
  (params (Key :type "Key Structure"))
  ; Normal Movement
  (:`Pressed`
    (if (`self.IsPlayerInside`) :!label _label_6
      (if (> (`self.ForwardOffSet`) 0.0)
        (goto _label_5)
        (else
          (goto _label_5 :!via `Reverse`)))))
  (:`Released`
    (goto _label_5 :!via `Stop`)))

(event `EnhancedInput|/Game/VRE/Input/Actions/MotionControllerThumbRight_Y`
  (params (ActionValue :type "Float (double-precision)") (ElapsedSeconds :type "Float (double-precision)") (TriggeredSeconds :type "Float (double-precision)") (InputAction :type "InputAction Object Reference" :default "/Game/VRE/Input/Actions/MotionControllerThumbRight_Y.MotionControllerThumbRight_Y"))
  (bind _returnvalue (> ActionValue 0.75))
  (bind _returnvalue_2 (< ActionValue -0.75))
  ; Normal Movement
  (:`Triggered`
    (`|ExecutionSequence`
      (:`then_0`
        (if _returnvalue
          (goto _label_6)
          (else
            (if (`KismetMathLibrary.BooleanNOR` _returnvalue _returnvalue_2) :!label _label_7
              (goto _label_5 :!via `Stop`)))))
      (:`then_1`
        (if _returnvalue_2
          (if (`self.IsPlayerInside`) :!label _label_8
            (if (> (`self.ForwardOffSet`) 0.0)
              (goto _label_5 :!via `Reverse`)
              (else
                (goto _label_5))))
          (else
            (goto _label_7))))))
  (:`Completed`
    (goto _label_5 :!via `Stop`)))

(event `Key|M`
  (params (Key :type "Key Structure"))
  ; Normal Movement
  (:`Pressed`
    (goto _label_8))
  (:`Released`
    (goto _label_5 :!via `Stop`)))

(event `self.Box.OnComponentBeginOverlap`
  (params (OverlappedComponent :type "PrimitiveComponent Object Reference") (OtherActor :type "Actor Object Reference") (OtherComp :type "PrimitiveComponent Object Reference") (OtherBodyIndex :type Integer) (bFromSweep :type Boolean) (SweepResult :type "HitResult Structure (by ref)"))
  ; Player Hit Detection
  (bind _asbp_vrcharacter (cast `/Game/VRE/Core/Character/BP_VRCharacter` OtherActor))
  (if (== (`/Game/VRE/Core/Character/BP_VRCharacter.Body` _asbp_vrcharacter) OtherComp)
    (set `self.IsPlayerInside` true)))

(event `self.Box.OnComponentEndOverlap`
  (params (OverlappedComponent :type "PrimitiveComponent Object Reference") (OtherActor :type "Actor Object Reference") (OtherComp :type "PrimitiveComponent Object Reference") (OtherBodyIndex :type Integer))
  ; Player Hit Detection
  (bind _asbp_vrcharacter (cast `/Game/VRE/Core/Character/BP_VRCharacter` OtherActor))
  (if (== (`/Game/VRE/Core/Character/BP_VRCharacter.Body` _asbp_vrcharacter) OtherComp)
    (set `self.IsPlayerInside` false)))

(fn `UserConstructionScript`)