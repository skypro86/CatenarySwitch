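; Contact wire clamp Blueprint for the catenary switch, extending a parent class that supplies the core behavior.
; Tick gates the parent's Tick: clamps flagged IsFirst always run it, while others require CheckCorrectHeight at Socket_Clamp3 to pass.
; That check runs on the actor GetActorOfClass finds for this same clamp class, looked up every frame.
; A similar powerline holder height check is left unconnected and never runs.
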(event `self.ReceiveTick`
  (params (DeltaSeconds :type "Float (single-precision)"))
  (if (`self.IsFirst`)
    (`parent.ReceiveTick` DeltaSeconds :!label _label)
    (else
      (bind _returnvalue (`GameplayStatics.GetActorOfClass` "BP_Clamp_ContactWire_C"))
      (bind _iscorrect (`self.CheckCorrectHeight` _returnvalue "Socket_Clamp3" (`/Game/CatenarySwitch/Core/BP_HoldableBase.GrippableStaticMesh` _returnvalue)))
      (if _iscorrect
        (goto _label)))))

(fn `UserConstructionScript`
  (`parent.UserConstructionScript`))