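; BP_Switch_Movable is the moving part of a catenary switch, built on a parent class with a grippable mesh.
; F plays a timeline that lerps the mesh's relative rotation between StartRot and EndRot, and G reverses it.
; Tick sets those rotations once whenever the movable socket's height check becomes true.
; Parent Tick runs only while the BP_Switch_Fixed actor, looked up every frame, passes its own height check.
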(event `Key|F`
  (params (Key :type "Key Structure"))
  (:`Pressed`
    (bind (_direction _newtrack_0) (`Timeline|Timeline` :`NewTime` 5.0 :!via `PlayFromStart` :!label _label)
      (:`Update`
        (`SceneComponent.K2_SetRelativeRotation` (`self.GrippableStaticMesh`) (`KismetMathLibrary.RLerp` (`self.StartRot`) (`self.EndRot`) _newtrack_0) false false)))))

(event `Key|G`
  (params (Key :type "Key Structure"))
  (:`Pressed`
    (goto _label :!via `Reverse`)))

(event `self.ReceiveTick`
  (params (DeltaSeconds :type "Float (single-precision)"))
  (`|ExecutionSequence`
    (:`then_0`
      (bind _iscorrect (`self.CheckCorrectHeight` "Socket_Switch_Movable" (`self.GrippableStaticMesh`)))
      (if _iscorrect
        (`/Engine/EditorBlueprintResources/StandardMacros.DoOnce` false :!label _label_2
          (:`Completed`
            (set `self.StartRot` (struct :`Yaw` 180.0))
            (set `self.EndRot` (struct :`Pitch` -45.0 :`Yaw` 180.0))))
        (else
          (goto _label_2 :!via `Reset`))))
    (:`then_1`
      (bind _returnvalue (`GameplayStatics.GetActorOfClass` "/Game/CatenarySwitch/Art/Industrial/CatenarySwitch/Blueprints/BP_Switch_Fixed.BP_Switch_Fixed_C"))
      (bind _iscorrect_2 (`self.CheckCorrectHeight` _returnvalue "Socket_Switch_Fixed" (`/Game/CatenarySwitch/Core/BP_HoldableBase.GrippableStaticMesh` _returnvalue)))
      (if _iscorrect_2
        (`parent.ReceiveTick` DeltaSeconds)))))

(event `self.ReceiveBeginPlay`
  (`parent.ReceiveBeginPlay`))

(fn `UserConstructionScript`
  (`parent.UserConstructionScript`))