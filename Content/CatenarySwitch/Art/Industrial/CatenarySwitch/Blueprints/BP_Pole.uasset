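; Pole actor for a catenary switch installation, carrying the switch box, switch parts, clamps, cable protectors and other mounted components.
; The construction script offsets three boxes and two clamps by MoveDistance, positive for IsLeft and negated for IsRight.
; On BeginPlay, Setup fills the CorrectHeightCollection map, pairing socket names with their matching components.
; Nothing in this graph reads that map.
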(event `self.ReceiveBeginPlay`
  (`self.Setup`))

(fn `Setup`
  (`|ExecutionSequence`
    (:`then_0`
      (`BlueprintMapLibrary.Map_Add` (`self.CorrectHeightCollection`) "Socket_HM_Bottom" (`self.HM_Bottom`))
      (`BlueprintMapLibrary.Map_Add` (`self.CorrectHeightCollection`) "Socket_HM_Top" (`self.HM_Top`))
      (`BlueprintMapLibrary.Map_Add` (`self.CorrectHeightCollection`) "Socket_SwitchBox" (`self.SwitchBox`))
      (`BlueprintMapLibrary.Map_Add` (`self.CorrectHeightCollection`) "Socket_SR_Bottom" (`self.SR_Bottom`)))
    (:`then_1`
      (`BlueprintMapLibrary.Map_Add` (`self.CorrectHeightCollection`) "Socket_MB_CableProtector1" (`self.MB_CableProtector1`))
      (`BlueprintMapLibrary.Map_Add` (`self.CorrectHeightCollection`) "Socket_MB_CableProtector2" (`self.MB_CableProtector2`))
      (`BlueprintMapLibrary.Map_Add` (`self.CorrectHeightCollection`) "Socket_PC_Protector" (`self.PC_Protector`))
      (`BlueprintMapLibrary.Map_Add` (`self.CorrectHeightCollection`) "Socket_GroundingCable" (`self.GroundingCable`))
      (`BlueprintMapLibrary.Map_Add` (`self.CorrectHeightCollection`) "Socket_PowerCable" (`self.PowerCable`)))
    (:`then_2`
      (`BlueprintMapLibrary.Map_Add` (`self.CorrectHeightCollection`) "Socket_MB_Right1" (`self.MB_Right1`))
      (`BlueprintMapLibrary.Map_Add` (`self.CorrectHeightCollection`) "Socket_MB_Right2" (`self.MB_Right2`))
      (`BlueprintMapLibrary.Map_Add` (`self.CorrectHeightCollection`) "Socket_MB_Right3" (`self.MB_Right3`))
      (`BlueprintMapLibrary.Map_Add` (`self.CorrectHeightCollection`) "Socket_MB_Right4" (`self.MB_Right4`))
      (`BlueprintMapLibrary.Map_Add` (`self.CorrectHeightCollection`) "Socket_MB_Right5" (`self.MB_Right5`))
      (`BlueprintMapLibrary.Map_Add` (`self.CorrectHeightCollection`) "Socket_MB_Right6" (`self.MB_Right6`))
      (`BlueprintMapLibrary.Map_Add` (`self.CorrectHeightCollection`) "Socket_MB_Right7" (`self.MB_Right7`)))
    (:`then_3`
      (`BlueprintMapLibrary.Map_Add` (`self.CorrectHeightCollection`) "Socket_MB_SwitchCable1" (`self.MB_SwitchCable1`))
      (`BlueprintMapLibrary.Map_Add` (`self.CorrectHeightCollection`) "Socket_MB_SwitchCable2" (`self.MB_SwitchCable2`))
      (`BlueprintMapLibrary.Map_Add` (`self.CorrectHeightCollection`) "Socket_MB_SwitchCable3" (`self.MB_SwitchCable3`)))
    (:`then_4`
      (`BlueprintMapLibrary.Map_Add` (`self.CorrectHeightCollection`) "Socket_MB_Left1" (`self.MB_Left1`))
      (`BlueprintMapLibrary.Map_Add` (`self.CorrectHeightCollection`) "Socket_MB_Left2" (`self.MB_Left2`))
      (`BlueprintMapLibrary.Map_Add` (`self.CorrectHeightCollection`) "Socket_MB_Left3" (`self.MB_Left3`))
      (`BlueprintMapLibrary.Map_Add` (`self.CorrectHeightCollection`) "Socket_MB_LeftTurned" (`self.MB_LeftTurned`))
      (`BlueprintMapLibrary.Map_Add` (`self.CorrectHeightCollection`) "Socket_MB_Left_Top" (`self.MB_Left_Top`))
      (`BlueprintMapLibrary.Map_Add` (`self.CorrectHeightCollection`) "Socket_Grounding_Insulator" (`self.Grounding_Insulator`)))
    (:`then_5`
      (`BlueprintMapLibrary.Map_Add` (`self.CorrectHeightCollection`) "Socket_Switch_Fixed" (`self.Switch_Fixed`))
      (`BlueprintMapLibrary.Map_Add` (`self.CorrectHeightCollection`) "Socket_Switch_Movable" (`self.Switch_Movable`))
      (`BlueprintMapLibrary.Map_Add` (`self.CorrectHeightCollection`) "Socket_SR_Top" (`self.SR_Top`))
      (`BlueprintMapLibrary.Map_Add` (`self.CorrectHeightCollection`) "Socket_Powerline_Holder" (`self.Powerline_Holder`)))
    (:`then_6`
      (`BlueprintMapLibrary.Map_Add` (`self.CorrectHeightCollection`) "Socket_Clamp1" (`self.Clamp1`))
      (`BlueprintMapLibrary.Map_Add` (`self.CorrectHeightCollection`) "Socket_Clamp2" (`self.Clamp2`))
      (`BlueprintMapLibrary.Map_Add` (`self.CorrectHeightCollection`) "Socket_Clamp3" (`self.Clamp3`))
      (`BlueprintMapLibrary.Map_Add` (`self.CorrectHeightCollection`) "Socket_Clamp4" (`self.Clamp4`)))))

(fn `UserConstructionScript`
  (if (`self.IsLeft`)
    (`SceneComponent.K2_AddLocalOffset` (`self.Box36`) (`KismetMathLibrary.MakeVector` (`self.MoveDistance`)) false false)
    (`SceneComponent.K2_AddLocalOffset` (`self.Box38`) (`KismetMathLibrary.MakeVector` (`self.MoveDistance`)) false false)
    (`SceneComponent.K2_AddLocalOffset` (`self.Box34`) (`KismetMathLibrary.MakeVector` (`self.MoveDistance`)) false false)
    (`SceneComponent.K2_AddLocalOffset` (`self.Clamp1`) (`KismetMathLibrary.MakeVector` (`self.MoveDistance`)) false false)
    (`SceneComponent.K2_AddLocalOffset` (`self.Clamp2`) (`KismetMathLibrary.MakeVector` (`self.MoveDistance`)) false false)
    (elif (`self.IsRight`)
      (`SceneComponent.K2_AddLocalOffset` (`self.Box36`) (`KismetMathLibrary.MakeVector` (* (`self.MoveDistance`) -1.0)) false false)
      (`SceneComponent.K2_AddLocalOffset` (`self.Box38`) (`KismetMathLibrary.MakeVector` (* (`self.MoveDistance`) -1.0)) false false)
      (`SceneComponent.K2_AddLocalOffset` (`self.Box34`) (`KismetMathLibrary.MakeVector` (* (`self.MoveDistance`) -1.0)) false false)
      (`SceneComponent.K2_AddLocalOffset` (`self.Clamp1`) (`KismetMathLibrary.MakeVector` (* (`self.MoveDistance`) -1.0)) false false)
      (`SceneComponent.K2_AddLocalOffset` (`self.Clamp2`) (`KismetMathLibrary.MakeVector` (* (`self.MoveDistance`) -1.0)) false false))))