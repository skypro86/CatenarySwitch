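; BP_PowerCable is the power cable in the catenary switch assembly, gating its inherited Tick behavior on the placement of two other parts.
; Each Tick looks up BP_PC_Protector and BP_MB_Left_Top by class and calls CheckCorrectHeight on each with its socket name and grippable mesh.
; Parent Tick runs only when both checks pass, so the cable's own per-frame logic lives in the parent class.
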(event `self.ReceiveTick`
  (params (DeltaSeconds :type "Float (single-precision)"))
  (bind _returnvalue (`GameplayStatics.GetActorOfClass` "/Game/CatenarySwitch/Art/Industrial/CatenarySwitch/Blueprints/BP_PC_Protector.BP_PC_Protector_C"))
  (bind _iscorrect (`self.CheckCorrectHeight` _returnvalue "Socket_PC_Protector" (`/Game/CatenarySwitch/Core/BP_HoldableBase.GrippableStaticMesh` _returnvalue)))
  (bind _returnvalue_2 (`GameplayStatics.GetActorOfClass` "/Game/CatenarySwitch/Art/Industrial/CatenarySwitch/Blueprints/BP_MB_Left_Top.BP_MB_Left_Top_C"))
  (bind _iscorrect_2 (`self.CheckCorrectHeight` _returnvalue_2 "Socket_MB_Left_Top" (`/Game/CatenarySwitch/Core/BP_HoldableBase.GrippableStaticMesh` _returnvalue_2)))
  (if (and _iscorrect_2 _iscorrect)
    (`parent.ReceiveTick` DeltaSeconds)))

(fn `UserConstructionScript`
  (`parent.UserConstructionScript`))