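; BP_MB_Left2 is a child Blueprint in the CatenarySwitch industrial art set that makes its per-frame behavior depend on BP_MB_Left1.
; Each Tick it looks up BP_MB_Left1 and calls CheckCorrectHeight with that actor's grippable mesh and socket Socket_MB_Left1.
; The parent Tick runs only while that check passes, so this part's inherited logic waits on Left1 being at the correct height.
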(event `self.ReceiveTick`
  (params (DeltaSeconds :type "Float (single-precision)"))
  (bind _returnvalue (`GameplayStatics.GetActorOfClass` "/Game/CatenarySwitch/Art/Industrial/CatenarySwitch/Blueprints/BP_MB_Left1.BP_MB_Left1_C"))
  (bind _iscorrect (`self.CheckCorrectHeight` _returnvalue "Socket_MB_Left1" (`/Game/CatenarySwitch/Core/BP_HoldableBase.GrippableStaticMesh` _returnvalue)))
  (if _iscorrect
    (`parent.ReceiveTick` DeltaSeconds)))

(fn `UserConstructionScript`
  (`parent.UserConstructionScript`))