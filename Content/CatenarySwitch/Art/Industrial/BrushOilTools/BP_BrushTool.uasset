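; BP_BrushTool is a grippable brush that swaps the end segments of a BP_Cable to a brushed material on contact.
; Each tick, a sphere trace detects hits on the cable's first or last section and changes those spline mesh materials.
; In tutorial levels it starts hidden without collision, appearing once a contact-wire clamp passes its height check.
; A looping timer resets the brush to its starting transform when it falls too low.
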(event `self.ReceiveBeginPlay`
  (bind _grippablestaticmesh (`self.GrippableStaticMesh`))
  (bind _grippablestaticmesh_2 (`self.GrippableStaticMesh`))
  ; Setup & Set Visibility
  (set `self.Position` (`SceneComponent.K2_GetComponentLocation` _grippablestaticmesh_2))
  (set `self.Rotation` (`SceneComponent.K2_GetComponentRotation` _grippablestaticmesh_2))
  (`KismetSystemLibrary.K2_SetTimer` null "HeightCheck" 0.1 true)
  (bind _returnvalue (`GameplayStatics.GetCurrentLevelName` true))
  (if (or (`KismetStringLibrary.EqualEqual_StrStr` _returnvalue "Switch_Easy") (`KismetStringLibrary.EqualEqual_StrStr` _returnvalue "Switch_Easy_TiltedLeft") (`KismetStringLibrary.EqualEqual_StrStr` _returnvalue "Switch_Easy_TiltedRight"))
    (`SceneComponent.SetVisibility` _grippablestaticmesh false true)
    (`PrimitiveComponent.SetCollisionEnabled` _grippablestaticmesh "NoCollision")))

(event `self.ReceiveTick`
  (params (DeltaSeconds :type "Float (single-precision)"))
  (bind _grippablestaticmesh (`self.GrippableStaticMesh`))
  (bind _brushedmaterial (`self.BrushedMaterial`))
  (bind _returnvalue (`SceneComponent.K2_GetComponentLocation` (`self.GrippableStaticMesh`)))
  (`|ExecutionSequence`
    (:`then_0`
      ; Checks if tutorialLevel & spawns tools at correct time
      (bind _returnvalue_2 (`GameplayStatics.GetCurrentLevelName` true))
      (if (or (`KismetStringLibrary.EqualEqual_StrStr` _returnvalue_2 "Switch_Easy") (`KismetStringLibrary.EqualEqual_StrStr` _returnvalue_2 "Switch_Easy_TiltedLeft") (`KismetStringLibrary.EqualEqual_StrStr` _returnvalue_2 "Switch_Easy_TiltedRight"))
        (bind _outactors (`GameplayStatics.GetAllActorsOfClass` "/Game/CatenarySwitch/Art/Industrial/Clamps/BP_Clamp_ContactWire.BP_Clamp_ContactWire_C"))
        (bind _output (`|GetArrayItem` _outactors 1))
        (bind _iscorrect (`/Game/CatenarySwitch/Core/BP_HoldableBase.CheckCorrectHeight` _output "Socket_Clamp4" (`/Game/CatenarySwitch/Core/BP_HoldableBase.GrippableStaticMesh` _output)))
        (if _iscorrect
          (`/Engine/EditorBlueprintResources/StandardMacros.DoOnce` false
            (:`Completed`
              (`SceneComponent.SetVisibility` _grippablestaticmesh true true)
              (`PrimitiveComponent.SetCollisionEnabled` _grippablestaticmesh "QueryAndPhysics"))))))
    (:`then_1`
      ; CableHit Check
      (bind (_outhit _returnvalue_3) (`KismetSystemLibrary.SphereTraceSingle` _returnvalue _returnvalue 10.0 "TraceTypeQuery1"))
      (if _returnvalue_3
        (bind (_bblockinghit _binitialoverlap _time _distance _location _impactpoint _normal _impactnormal _physmat _hitactor _hitcomponent) (`GameplayStatics.BreakHitResult` _outhit))
        (bind _asbp_cable (cast `/Game/CatenarySwitch/Art/Industrial/Cable/BP_Cable` _hitactor))
        (bind _links (`/Game/CatenarySwitch/Art/Industrial/Cable/BP_Cable.Links` _asbp_cable))
        (if (== (`|GetArrayItem` _links) _hitcomponent)
          (bind _splinemeshsegments (`/Game/CatenarySwitch/Art/Industrial/Cable/BP_Cable.SplineMeshSegments` _asbp_cable))
          (`PrimitiveComponent.SetMaterial` (`|GetArrayItem` _splinemeshsegments) 0 _brushedmaterial)
          (elif (== (`|GetArrayItem` _links (- (`/Game/CatenarySwitch/Art/Industrial/Cable/BP_Cable.NumLinks` _asbp_cable) 2)) _hitcomponent)
            (bind _numlinks (`/Game/CatenarySwitch/Art/Industrial/Cable/BP_Cable.NumLinks` _asbp_cable))
            (`PrimitiveComponent.SetMaterial` (`|GetArrayItem` _splinemeshsegments (- _numlinks 1)) 0 _brushedmaterial)
            (`PrimitiveComponent.SetMaterial` (`|GetArrayItem` _splinemeshsegments (- _numlinks 2)) 0 _brushedmaterial)))))))

(event `HeightCheck`
  (bind _grippablestaticmesh (`self.GrippableStaticMesh`))
  (bind (_returnvalue_x _returnvalue_y _returnvalue_z) (`KismetMathLibrary.BreakVector` (`SceneComponent.K2_GetComponentLocation` (`self.GrippableStaticMesh`))))
  ; Custom Event to resapwn the object if below a certain thershold
  (if (< _returnvalue_z 120.0)
    (`PrimitiveComponent.SetPhysicsLinearVelocity` _grippablestaticmesh (0.0 0.0 0.0) false "None")
    (`PrimitiveComponent.SetPhysicsAngularVelocityInRadians` _grippablestaticmesh (0.0 0.0 0.0) false "None")
    (`SceneComponent.K2_SetWorldLocation` _grippablestaticmesh (`self.Position`) false false)
    (`SceneComponent.K2_SetWorldRotation` _grippablestaticmesh (`self.Rotation`) false false)))

(fn `UserConstructionScript`)